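; BP_SphereSpawner is a spawner actor that periodically creates actors of a configurable SphereClass at random positions around itself.
; On BeginPlay it starts a looping timer that calls SpawnSphere every SpawnInterval.
; Each call randomizes X and Y within SpawnAreaExtent around the actor's location.
; Z comes directly from SpawnHeight as an absolute world height, independent of the spawner's own height.
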(event `self.ReceiveBeginPlay`
  (`KismetSystemLibrary.K2_SetTimer` null "SpawnSphere" (`self.SpawnInterval`) true))

(fn `SpawnSphere`
  (bind _x (.x (`self.SpawnAreaExtent`)))
  (bind _y (.y (`self.SpawnAreaExtent`)))
  (`|SpawnActorFromClass` (`self.SphereClass`) (`KismetMathLibrary.Conv_VectorToTransform` (`KismetMathLibrary.MakeVector` (.x (+ (`KismetMathLibrary.MakeVector` (`KismetMathLibrary.RandomFloatInRange` (* _x -1.0) _x) (`KismetMathLibrary.RandomFloatInRange` (* _y -1.0) _y)) (`self.K2_GetActorLocation`))) (.y (+ (`KismetMathLibrary.MakeVector` (`KismetMathLibrary.RandomFloatInRange` (* _x -1.0) _x) (`KismetMathLibrary.RandomFloatInRange` (* _y -1.0) _y)) (`self.K2_GetActorLocation`))) (`self.SpawnHeight`))) "Undefined" "MultiplyWithRoot" null null))

(fn `UserConstructionScript`)