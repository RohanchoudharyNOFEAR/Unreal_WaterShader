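; BP_Water is a water plane that spawns a ripple where an actor begins overlapping its trigger.
; On BeginPlay it clears the ripple render target, creates dynamic instances of the ripple-draw and water materials, and applies the water one to the mesh.
; AddRipple converts the actor's world position into plane UVs, passes that center to both materials, and draws the ripple material with a radius into the render target.
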(event `self.WaterTrigger.OnComponentBeginOverlap`
  (params (OverlappedComponent :type "PrimitiveComponent Object Reference") (OtherActor :type "Actor Object Reference") (OtherComp :type "PrimitiveComponent Object Reference") (OtherBodyIndex :type Integer) (bFromSweep :type Boolean) (SweepResult :type "HitResult Structure (by ref)"))
  (`self.AddRipple` (`self.K2_GetActorLocation` OtherActor)))

(event `self.ReceiveBeginPlay`
  (bind _returnvalue (`KismetMaterialLibrary.CreateDynamicMaterialInstance` "/Game/Shaders/Water/M_DrawRipple.M_DrawRipple"))
  (set `self.RippleDrawMID` _returnvalue)
  (`KismetRenderingLibrary.ClearRenderTarget2D` (`self.RT_Ripples`))
  (bind _returnvalue_2 (`KismetMaterialLibrary.CreateDynamicMaterialInstance` "/Game/Shaders/Water/M_Water.M_Water"))
  (set `self.WaterMID` _returnvalue_2)
  (`PrimitiveComponent.SetMaterial` (`self.StaticMeshComponent`) 0 _returnvalue_2))

(event `self.ReceiveTick`
  (params (DeltaSeconds :type "Float (single-precision)")))

(fn `AddRipple`
  (params (WorldPos :type "Vector Structure"))
  (bind _output_get (set `self.CenterUV` (`KismetMathLibrary.MakeVector2D` (+ (/ (.x (`KismetMathLibrary.InverseTransformLocation` (`SceneComponent.K2_GetComponentToWorld` (`self.StaticMeshComponent`)) WorldPos)) (`self.PlaneSize`)) 0.5) (+ (/ (.y (`KismetMathLibrary.InverseTransformLocation` (`SceneComponent.K2_GetComponentToWorld` (`self.StaticMeshComponent`)) WorldPos)) (`self.PlaneSize`)) 0.5))))
  (bind (_x _y) (`KismetMathLibrary.BreakVector2D` _output_get))
  (bind _linearcolor (make `LinearColor` _x _y 0.0 1.0))
  (`MaterialInstanceDynamic.SetVectorParameterValue` (`self.WaterMID`) "CenterUV" _linearcolor)
  (`MaterialInstanceDynamic.SetVectorParameterValue` (`self.RippleDrawMID`) "CenterUV" _linearcolor)
  (`MaterialInstanceDynamic.SetScalarParameterValue` (`self.RippleDrawMID`) "Radius" (`self.RippleRadius`))
  (`KismetRenderingLibrary.DrawMaterialToRenderTarget` (`self.RT_Ripples`) (`self.RippleDrawMID`)))

(fn `UserConstructionScript`)